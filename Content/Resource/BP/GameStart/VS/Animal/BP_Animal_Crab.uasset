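; Crab animal actor that walks through the scene and marks any mouse actor it overlaps as dead.
; On ready it plays a one-shot intro animation that leads into the walk animation, and sets a short lifespan.
; The end of animation playback enables walking, while water and ground events switch between the in-water and land walk animations.
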(event `self.OnOverlapWidgtMouse`
  (params (MouseActor :type "MouseActor Object Reference"))
  (`MouseActor.SetMouseDeath` MouseActor true))

(event `self.OnReady`
  (`FlipbookBaseComponent.SetPlayAnimationOnce` (`self.M_Actor`) "/Game/Resource/Texture/Sprite/VS/Map/Animal/Water/PF_Animal_Crab_Ready.PF_Animal_Crab_Ready" "/Game/Resource/Texture/Sprite/VS/Map/Animal/Water/PF_Animal_Crab_Walk.PF_Animal_Crab_Walk")
  (`self.SetLifeSpan` 6.8))

(event `self.OnAnimationPlayEnd`
  (`self.EnableWalk`))

(event `self.OnInWater`
  (`FlipbookBaseComponent.SetPlayAnimation` (`self.M_Actor`) "/Game/Resource/Texture/Sprite/VS/Map/Animal/Water/PF_Animal_Crab_WalkInWater.PF_Animal_Crab_WalkInWater" false))

(event `self.OnGround`
  (`FlipbookBaseComponent.SetPlayAnimation` (`self.M_Actor`) "/Game/Resource/Texture/Sprite/VS/Map/Animal/Water/PF_Animal_Crab_Walk.PF_Animal_Crab_Walk" false))

(fn `UserConstructionScript`)