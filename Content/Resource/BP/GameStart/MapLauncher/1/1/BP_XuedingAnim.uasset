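; BP_XuedingAnim is a map actor that gives MouseActors on its row a short acceleration buff and controls its own visibility.
; A looping timer, cleared on destroy, runs a small sphere trace just below the actor, applying the buff and setting a Mouse flag when the hit mouse's row matches.
; Tick hides the actor only while its card count is zero and that flag is false.
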(event `self.ReceiveTick`
  (params (DeltaSeconds :type "Float (single-precision)"))
  (bind _returnvalue (`self.GetCardNums`))
  (if (== _returnvalue 0)
    (if (`self.bMouse`)
      (`self.SetActorHiddenInGame` false)
      (else
        (`self.SetActorHiddenInGame` true)))
    (else
      (`self.SetActorHiddenInGame` false))))

(event `self.ReceiveDestroyed`
  (`KismetSystemLibrary.K2_ClearAndInvalidateTimerHandle` (`self.TimerHd`)))

(event `self.ReceiveBeginPlay`
  (bind _returnvalue (`KismetSystemLibrary.K2_SetTimerDelegate` (delegate `OnMouseEnter`) 0.2 true))
  (set `self.TimerHd` _returnvalue))

(event `OnMouseEnter`
  (bind _returnvalue (- (`self.K2_GetActorLocation`) (0.0 0.0 7.0)))
  (bind _outhit (`KismetSystemLibrary.SphereTraceSingle` :`Start` _returnvalue :`End` _returnvalue :`Radius` 27.0 :`TraceChannel` "TraceTypeQuery11" :`DrawDebugType` "ForOneFrame"))
  (bind _asmouse_actor (cast `MouseActor` (`.HitActor` (`GameplayStatics.BreakHitResult` _outhit)))
    (:`then`
      (bind _returnvalue_2 (`MouseActor.GetMouseLine` _asmouse_actor))
      (bind _returnvalue_3 (`self.GetLine`))
      (if (== (`.Row` (break `Line` _returnvalue_3)) (`.Row` (break `Line` _returnvalue_2)))
        (set `self.bMouse` true)
        (`MouseActor.AddAccelerateBuff` _asmouse_actor 0.25)
        (else
          (set `self.bMouse` false))))
    (:`CastFailed`
      (set `self.bMouse` false))))

(fn `UserConstructionScript`)